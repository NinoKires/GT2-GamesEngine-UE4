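; Base Blueprint for player projectiles, which damage the actor they overlap and then destroy themselves.
; The construction script creates a dynamic material instance, applies Scale to the Projectile component, and configures ProjectileMovement with Speed as max speed and zero initial speed.
; BeginPlay tints that material with ProjectileColour, and the overlap event applies Damage with no filtering of the other actor.
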(event `self.ReceiveBeginPlay`
  (`MaterialInstanceDynamic.SetVectorParameterValue` (`self.ProjectileMaterial`) "Colour" (`self.ProjectileColour`)))

(event `self.Projectile.OnComponentBeginOverlap`
  (params (OverlappedComponent :type "PrimitiveComponent Object Reference") (OtherActor :type "Actor Object Reference") (OtherComp :type "PrimitiveComponent Object Reference") (OtherBodyIndex :type Integer) (bFromSweep :type Boolean) (SweepResult :type "HitResult Structure (by ref)"))
  (`GameplayStatics.ApplyDamage` OtherActor (`self.Damage`))
  (`self.K2_DestroyActor`))

(fn `UserConstructionScript`
  (bind _projectilemovement (`self.ProjectileMovement`))
  (bind _returnvalue (`PrimitiveComponent.CreateDynamicMaterialInstance` (`self.Projectile`) 0 null "None"))
  (set `self.ProjectileMaterial` _returnvalue)
  (`SceneComponent.SetWorldScale3D` (`self.Projectile`) (`self.Scale`))
  (set `ProjectileMovementComponent.MaxSpeed` (`self.Speed`) _projectilemovement)
  (set `ProjectileMovementComponent.InitialSpeed` 0.0 _projectilemovement))