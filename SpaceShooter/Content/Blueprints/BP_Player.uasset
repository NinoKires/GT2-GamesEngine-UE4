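; Player pawn for a shooter that moves on the X-Z plane, with a rising spin-in spawn animation that unlocks firing when finished.
; Axis input eases horizontal and vertical speeds, which Tick applies as swept moves while tilting the mesh, and box hits bounce them off the surface normal.
; Looping timers auto-fire single primary and twin secondary projectiles while held.
; Damage shakes the camera, and death explodes and triggers game over.
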(event `self.ReceiveBeginPlay`
  (bind _spawnlocation (`self.SpawnLocation`))
  ;[1 1 1] PlayerSpawnAnimation
  (bind _asbp_game_mode (cast `/Game/Blueprints/BP_GameMode` (`GameplayStatics.GetGameMode`)))
  (set `self.BP_GameMode` _asbp_game_mode)
  (set `self.Yaw` (.yaw (`self.K2_GetActorRotation`)))
  (set `self.SpawnLocation` (`self.K2_GetActorLocation`))
  (bind (_direction _speed) (`Timeline|SpawnAnimation`)
    (:`Update`
      (`self.K2_SetActorLocation` (`KismetMathLibrary.VLerp` _spawnlocation (+ _spawnlocation (0.0 0.0 60.0)) _speed))
      (`SceneComponent.K2_SetRelativeRotation` (`self.PlayerMash`) (`KismetMathLibrary.RLerp` (struct) (`KismetMathLibrary.MakeRotator` 0.0 0.0 (+ (`self.Yaw`) (`self.SpawnSpinCount`))) _speed) false false))
    (:`Finished`
      (set `self.MoveEnabled` true))))

(event `self.ReceiveTick`
  (params (DeltaSeconds :type "Float (single-precision)"))
  (bind _playermash (`self.PlayerMash`))
  ;[1 1 1] Movement
  (set `self.DelteSeconds` DeltaSeconds)
  (`self.K2_SetActorLocation` (+ (`self.K2_GetActorLocation`) (`KismetMathLibrary.MakeVector` (`self.HozSpeed`))) true)
  (`self.K2_SetActorLocation` (+ (`self.K2_GetActorLocation`) (`KismetMathLibrary.MakeVector` 0.0 0.0 (`self.VertSpeed`))) true)
  (`/Engine/EditorBlueprintResources/StandardMacros.IsValid` self
    (:`Is Valid`
      (`SceneComponent.K2_SetRelativeRotation` _playermash (`KismetMathLibrary.RInterpTo_Constant` (`SceneComponent.RelativeRotation` _playermash) (`KismetMathLibrary.MakeRotator` 0.0 0.0 (+ (* (`self.HozSpeed`) -10.0) (`self.Yaw`))) (`self.DelteSeconds`) 80.0) false false))))

(event `InputAxis|MoveUp`
  (params (AxisValue :type "Float (single-precision)"))
  ;[1 1 1] PlayerInput
  (bind _returndirectionspeed (`self.Movement` AxisValue (`self.VertSpeed`)))
  (set `self.VertSpeed` _returndirectionspeed))

(event `InputAxis|MoveRight`
  (params (AxisValue :type "Float (single-precision)"))
  ;[1 1 1] PlayerInput
  (bind _returndirectionspeed (`self.Movement` AxisValue (`self.HozSpeed`)))
  (set `self.HozSpeed` _returndirectionspeed))

(event `InputAction|PrimaryFire`
  (params (Key :type "Key Structure"))
  ;[1 1 1] Primary Fire
  (:`Pressed`
    (if (`self.MoveEnabled`)
      (`KismetSystemLibrary.K2_SetTimer` null "PrimFire" 0.2 true)
      (`self.PrimaryFire` (`SceneComponent.K2_GetComponentToWorld` (`self.ProjectileSpawn`)) :!label _label)))
  (:`Released`
    (`KismetSystemLibrary.K2_ClearTimer` null "PrimFire")))

(event `PrimFire`
  ;[1 1 1] Primary Fire
  (goto _label))

(event `InputAction|SecondaryFire`
  (params (Key :type "Key Structure"))
  (:`Pressed`
    (if (`self.MoveEnabled`)
      (`KismetSystemLibrary.K2_SetTimer` null "SecFire" 0.6 true)
      (`self.Secondary Fire` (`SceneComponent.K2_GetComponentToWorld` (`self.ProjectileSpawnL`)) :!label _label_2)
      (`self.Secondary Fire` (`SceneComponent.K2_GetComponentToWorld` (`self.ProjectileSpawnR`)))))
  (:`Released`
    (`KismetSystemLibrary.K2_ClearTimer` null "SecFire")))

(event `SecFire`
  (goto _label_2))

(event `self.ReceiveAnyDamage`
  (params (Damage :type "Float (single-precision)") (DamageType :type "DamageType Object Reference") (InstigatedBy :type "Controller Object Reference") (DamageCauser :type "Actor Object Reference"))
  (bind _returnvalue (`self.K2_GetActorLocation`))
  (bind _bp_gamemode (`self.BP_GameMode`))
  (set `self.Health` (`KismetMathLibrary.FClamp` (- (`self.Health`) Damage) 0.0 (`self.MaxHealth`)))
  (`/Game/Blueprints/BP_GameMode.PlayCamShake` (`self.BP_GameMode`) "/Game/Blueprints/BP_CameraShakeSmall.BP_CameraShakeSmall_C" (`self.K2_GetActorLocation`))
  (if (<= (`self.Health`) 0.0)
    (`GameplayStatics.SpawnEmitterAtLocation` "/Game/Assets/Particles/P_Pixel_Explosion_Player.P_Pixel_Explosion_Player" _returnvalue)
    (`GameplayStatics.PlaySoundAtLocation` null _returnvalue (struct) 1.0 1.0 0.0 null null null)
    (`/Game/Blueprints/BP_GameMode.PlayCamShake` _bp_gamemode "/Game/Blueprints/BP_CameraShake.BP_CameraShake_C" (`self.K2_GetActorLocation`))
    (`/Game/Blueprints/BP_GameMode.GameOver` _bp_gamemode)
    (`self.K2_DestroyActor`)))

(event `self.Box.OnComponentHit`
  (params (HitComponent :type "PrimitiveComponent Object Reference") (OtherActor :type "Actor Object Reference") (OtherComp :type "PrimitiveComponent Object Reference") (NormalImpulse :type "Vector Structure") (Hit :type "HitResult Structure (by ref)"))
  (set `self.HozSpeed` (* (* (`KismetMathLibrary.Abs` (`self.HozSpeed`)) 2.0) (.x Hit_Normal)))
  (set `self.VertSpeed` (* (* (`KismetMathLibrary.Abs` (`self.VertSpeed`)) 2.0) (.z Hit_Normal))))

(fn `Movement`
  (params (Direction :type "Float (double-precision)") (Speed :type "Float (double-precision)"))
  (returns (ReturnDirectionSpeed :type "Float (double-precision)"))
  (return (`KismetMathLibrary.FInterpTo` Speed (* (* (`self.MovementSpeed`) Direction) (`self.DelteSeconds`)) (`self.DelteSeconds`) 6.0)))

(fn `PrimaryFire`
  (params (SpawnTransform :type "Transform Structure"))
  (locals (`Projectile Colour` :type "LinearColor Structure" :default (struct :`G` 0.120158 :`B` 0.739583)))
  (`|SpawnActorFromClass` "/Game/Blueprints/Projectiles/BP_ProjectilePlayerPrimary.BP_ProjectilePlayerPrimary_C" SpawnTransform "AlwaysSpawn" "OverrideRootScale" null (`local.Projectile Colour`) self))

(fn `Secondary Fire`
  (params (Spawn :type "Transform Structure"))
  (locals (Colour :type "LinearColor Structure" :default (struct :`R` 0.677083)))
  (`|SpawnActorFromClass` "/Game/Blueprints/Projectiles/BP_ProjectilePlayerSecondary.BP_ProjectilePlayerSecondary_C" Spawn "AlwaysSpawn" "OverrideRootScale" null (`local.Colour`) null))

(fn `UserConstructionScript`
  (set `self.Health` (`self.MaxHealth`)))